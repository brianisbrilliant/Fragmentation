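; Debug actor that scrubs a movie sequence forward or backward from keyboard input.
; On BeginPlay it enables input for the first player controller and prints the controls.
; Pressing or releasing the 1 key sets a target end or start frame, and both feed one PlayTo call on the Sequence player.
; Tick prints the current playback frame on screen.
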(event EventTick
  (params (DeltaSeconds :type Float%20%28single-precision%29))
  (Development|PrintString (Utilities|String|ToString(Integer) (.value (.frame (Sequencer|Player|GetCurrentTime (.Sequence (Variables|Default|GetSequence)))))) true true "(R=1.000000,G=0.000000,B=0.547758,A=1.000000)" 0.0))

(event EventBeginPlay
  (Input|EnableInput (Game|GetPlayerController 0))
  (Development|PrintString "Press 1 to play movie sequence,  
let go of 1 to play in reverse."))

(event Input|KeyboardEvents|DebugKey1
  (params (Key :type Key%20Structure :default "None") (ActionValue :type Input%20Action%20Value%20Structure))
  (:Pressed
    (Variables|Default|SetDesired%20Frame%20Number 99)
    (Development|PrintString "starting")
    (Class|MovieSceneSequencePlayer|Playto (.Sequence (Variables|Default|GetSequence)) (Utilities|Struct|MakeMovieSceneSequencePlaybackParams (Utilities|Struct|MakeFrameTime (Utilities|Struct|MakeFrameNumber (Variables|Default|GetDesired%20Frame%20Number)) 0.0) 0.0 "" "(Hours=0,Minutes=0,Seconds=0,Frames=0,bDropFrameFormat=False)" "Frame" "Play" false) :!label _label))
  (:Released
    (Variables|Default|SetDesired%20Frame%20Number 0)
    (goto _label)))

(fn ConstructionScript)