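; BP_SwellCube is an actor whose cube repeatedly swells on its own time dilation.
; BeginPlay applies the TimeDilation variable as custom time dilation, sets the starting scale, then loops on a delay to call Swell.
; Swell plays a timeline, fed a small random value, that lerps cube scale from StartScale toward MaxScale and resets its time when finished.
; A global time dilation call is left unconnected.
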(event `self.ReceiveBeginPlay`
  (set `self.CustomTimeDilation` (`self.Time Dilation`))
  (`SceneComponent.SetRelativeScale3D` (`self.Cube`) (`self.StartScale`))
  (`KismetSystemLibrary.Delay` 2.0 :!label _label)
  (`self.Swell`)
  (goto _label))

(event `Swell`
  (bind (_direction _newtrack_0) (`Timeline|Timeline` :`NewTime` (`KismetMathLibrary.RandomFloatInRange` 0.0 0.1) :!label _label_2)
    (:`Update`
      (`SceneComponent.SetRelativeScale3D` (`self.Cube`) (`KismetMathLibrary.VLerp` (`self.StartScale`) (`self.MaxScale`) _newtrack_0)))
    (:`Finished`
      (goto _label_2 :!via `SetNewTime`))))

(fn `UserConstructionScript`)